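; BaseProjectile is a player projectile Blueprint whose flight is shaped by a timeline rather than constant velocity.
; On BeginPlay it caches the ProjectileMovement velocity and starting rotation, then plays the timeline.
; Each update scales the horizontal velocity by one track, replaces vertical velocity with another, and drives pitch from a third while keeping the initial roll and yaw.
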(event `self.ReceiveBeginPlay`
  (bind _projectilemovement (`self.ProjectileMovement`))
  (set `self.BaseVelocity` (`MovementComponent.Velocity` _projectilemovement))
  (bind _output_get (set `self.StartingRotation` (`self.K2_GetActorRotation` self)))
  (bind (_direction _projectilevelocityscalar _verticalmovement _rotation) (`Timeline|Timeline_0` :!via `PlayFromStart`)
    (:`Update`
      (set `MovementComponent.Velocity` (`KismetMathLibrary.MakeVector` (* _projectilevelocityscalar (.x (`self.BaseVelocity`))) (* _projectilevelocityscalar (.y (`self.BaseVelocity`))) (* _verticalmovement 100.0)) _projectilemovement)
      (`self.K2_SetActorRotation` self (`KismetMathLibrary.MakeRotator` (.roll _output_get) (* _rotation 3.0) (.yaw _output_get)) false))))

(fn `UserConstructionScript`)