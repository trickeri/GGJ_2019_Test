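; Player controller that switches the player between normal control and a configurator mode built around the TheConfigamurator_BP actor found at BeginPlay.
; Entering plays a FadeIn sequence, blends the view to the configurator and enables cursor, click and hover events.
; Left click flags the hovered configurator part as attached to the mouse.
; Back exits, playing FadeOut and notifying the character, then returning the view to it after a delay.
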(event `self.ReceiveBeginPlay`
  ;[1 1 1] BeginPlay
  (bind _outactors (`GameplayStatics.GetAllActorsOfClass` "/Game/Blueprints/TheConfigamurator/TheConfigamurator_BP.TheConfigamurator_BP_C"))
  (bind _asthe_configamurator_bp (cast `/Game/Blueprints/TheConfigamurator/TheConfigamurator_BP` (`|GetArrayItem` _outactors)))
  (set `self.TheConfigurator` _asthe_configamurator_bp))

(event `UpdatePartHoveredOver`
  (params (ConfiguratorPart :type "/Game/Blueprints/TheConfigamurator/ConfiguratorPart Object Reference") (isHovering :type Boolean))
  ;[1 0.7602 0.8976] Configurator Part Mouse Functions
  (set `self.ConfiguratorPartHoveredOver` ConfiguratorPart)
  (set `self.MouseIsHoveringOverPart` isHovering))

(event `InputAction|MouseLeftClick`
  (params (Key :type "Key Structure"))
  ;[1 0.7602 0.8976] Configurator Part Mouse Functions
  (:`Pressed`
    (if (`self.MouseIsHoveringOverPart`)
      (set `/Game/Blueprints/TheConfigamurator/ConfiguratorPart.IsAttachedtoMouse` true (`self.ConfiguratorPartHoveredOver`)))))

(event `InputAction|Back`
  (params (Key :type "Key Structure"))
  ;[1 0.3698 0.3698] Back Button
  (:`Pressed`
    (if (`|EnumEquality` (`self.PlayerControlMode`) "NewEnumerator1")
      (`self.ExitConfiguratorMode`))))

(event `EnterConfiguratorMode`
  ;[1 0.4547 0.8496] Configurator Functions
  (set `self.PlayerControlMode` "NewEnumerator1")
  (bind _outactor (`LevelSequencePlayer.CreateLevelSequencePlayer` "/Game/Sequencer/FadeIn.FadeIn"))
  (`MovieSceneSequencePlayer.Play` (`LevelSequenceActor.SequencePlayer` _outactor))
  (`self.SetViewTargetWithBlend` (`self.TheConfigurator`))
  (set `self.bShowMouseCursor` true)
  (set `self.bEnableMouseOverEvents` true)
  (set `self.bEnableClickEvents` true))

(event `ExitConfiguratorMode`
  ;[1 0.4547 0.8496] Configurator Functions
  (set `self.PlayerControlMode` "NewEnumerator0")
  (bind _outactor (`LevelSequencePlayer.CreateLevelSequencePlayer` "/Game/Sequencer/FadeOut.FadeOut"))
  (bind _sequenceplayer (`LevelSequenceActor.SequencePlayer` _outactor))
  (`MovieSceneSequencePlayer.Play` _sequenceplayer)
  (bind _asplayer_character_bp (cast `/Game/Blueprints/Player/PlayerCharacter_BP` (`self.K2_GetPawn`)))
  (`/Game/Blueprints/Player/PlayerCharacter_BP.ExitConfiguratorMode_Pawn` _asplayer_character_bp)
  (`KismetSystemLibrary.Delay` 1.5)
  (`MovieSceneSequencePlayer.Stop` _sequenceplayer)
  (bind _asplayer_character_bp_2 (cast `/Game/Blueprints/Player/PlayerCharacter_BP` (`self.K2_GetPawn`)))
  (`self.SetViewTargetWithBlend` _asplayer_character_bp_2))

(fn `UserConstructionScript`)