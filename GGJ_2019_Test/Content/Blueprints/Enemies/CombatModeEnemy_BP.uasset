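; Combat-mode enemy minion Blueprint that takes damage, shows a floating health bar and dies at zero health.
; IsHit subtracts damage from Health and writes the fraction, on a 100-point scale, to the EnemyHPBar widget cached at BeginPlay.
; At zero it sets IsDead on MeleeMinionAnimBP, then waits briefly before calling the kill event for removal.
; Tick rotates the health bar toward the player camera every frame.
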(event `self.ReceiveBeginPlay`
  ;[1 1 1] BeginPlay
  (bind _asenemy_hpbar (cast `/Game/UI/Enemies/EnemyHPBar` (`WidgetComponent.GetUserWidgetObject` (`self.HPBar`))))
  (bind _output_get (set `self.MinionHPBar` _asenemy_hpbar))
  (set `/Game/UI/Enemies/EnemyHPBar.HealthPercent` 1.0 _output_get))

(event `self.ReceiveTick`
  (params (DeltaSeconds :type "Float (single-precision)"))
  ;[1 1 1] Tick
  (`self.RotateHealthBarToPlayer`))

(event `IsHit`
  (params (DamageAmt :type "Float (double-precision)"))
  ;[1 1 1] IsHit / Takes damage
  (bind _output_get (set `self.Health` (- (`self.Health`) DamageAmt)))
  (bind _output_get_2 (set `/Game/UI/Enemies/EnemyHPBar.HealthPercent` (/ _output_get 100.0) (`self.MinionHPBar`)))
  (if (<= _output_get_2 0.0)
    (`self.MinionKilledPt1`)))

(event `MinionKilledPt1`
  ;[1 0.1354 0.1354] Minion Killed
  (bind _asmelee_minion_anim_bp (cast `/Game/Blueprints/Enemies/MeleeMinionAnimBP` (`SkeletalMeshComponent.GetAnimInstance` (`self.Mesh`))))
  (set `/Game/Blueprints/Enemies/MeleeMinionAnimBP.IsDead` true _asmelee_minion_anim_bp)
  (`KismetSystemLibrary.Delay` 4.0)
  (`self.MinionKilled_Event`))

(event `MinionKilled_Event`
  ;[1 0.1354 0.1354] Minion Killed
  (`self.K2_DestroyActor`))

(event `RotateHealthBarToPlayer`
  ;[1 1 1] Keep HP bar facing the camera
  (`SceneComponent.K2_SetWorldRotation` (`self.HPBar`) (`KismetMathLibrary.FindLookAtRotation` (`SceneComponent.K2_GetComponentLocation` (`self.HPBar`)) (`PlayerCameraManager.GetCameraLocation` (`GameplayStatics.GetPlayerCameraManager` 0))) false false))

(fn `UserConstructionScript`)