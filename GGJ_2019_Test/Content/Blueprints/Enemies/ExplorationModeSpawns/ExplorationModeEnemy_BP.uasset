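; ExplorationModeEnemy_BP is an exploration-mode enemy that sends the player into combat on overlap.
; Overlap with the player character switches the player controller to combat mode and writes this enemy's spawn count to the game instance as the combat room enemy number.
; It then calls ChangeLevel on the first CombatLevelChange actor found, passing the player, and destroys itself after a short delay.
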(event `self.ReceiveActorBeginOverlap`
  (params (OtherActor :type "Actor Object Reference"))
  ;[1 1 1] Begin Overlap with player, Enter Combat zone
  (if (== (`GameplayStatics.GetObjectClass` OtherActor) "/Game/Blueprints/Player/PlayerCharacter_BP.PlayerCharacter_BP_C")
    (bind _asplayer_character_bp (cast `/Game/Blueprints/Player/PlayerCharacter_BP` OtherActor))
    (bind _asplayer_controller_bp (cast `/Game/Blueprints/Player/PlayerController_BP` (`GameplayStatics.GetPlayerController` 0)))
    (`/Game/Blueprints/Player/PlayerController_BP.EnterCombatMode` _asplayer_controller_bp)
    (`self.SetEnemiesToSpawn`)
    (bind _outactors (`GameplayStatics.GetAllActorsOfClass` "/Game/Blueprints/Environment/CombatLevelChange.CombatLevelChange_C"))
    (`/Game/Blueprints/Environment/CombatLevelChange.ChangeLevel` (`|GetArrayItem` _outactors) _asplayer_character_bp)
    (`KismetSystemLibrary.Delay` 0.4)
    (`self.K2_DestroyActor`)))

(event `SetEnemiesToSpawn`
  ;[1 1 1] Set number of enemies to spawn
  (bind _asgame_instance_bp (cast `/Game/Blueprints/General/GameInstance_BP` (`GameplayStatics.GetGameInstance`)))
  (set `/Game/Blueprints/General/GameInstance_BP.CombatRoomEnemyNumbers` (`self.NumberOfEnemiesToSpawn`) _asgame_instance_bp))

(fn `UserConstructionScript`)