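; ConfiguratorPart is an actor for a configurator part that can follow the mouse cursor until it is attached.
; While attached to the mouse, Tick deprojects the cursor, runs a short Visibility line trace and moves the actor to the hit location.
; Cursor-over events on the Part component report hover changes to PlayerController_BP.
; AttachPart clears the mouse-follow and hover flags, leaving the part in place.
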(event `self.ReceiveTick`
  (params (DeltaSeconds :type "Float (single-precision)"))
  (bind (_worldlocation _worlddirection) (`PlayerController.DeprojectMousePositionToWorld` (`GameplayStatics.GetPlayerController` 0)))
  ;[1 1 1] Tick
  (if (`self.IsAttachedtoMouse`)
    (bind _outhit (`KismetSystemLibrary.LineTraceSingle` _worldlocation (+ _worldlocation (* _worlddirection 1000.0)) "TraceTypeQuery1"))
    (if true
      (`self.K2_SetActorLocation` (+ (`.Location` (`GameplayStatics.BreakHitResult` _outhit)) (0.0 0.0 0.0))))))

(event `self.Part.OnBeginCursorOver`
  (params (TouchedComponent :type "PrimitiveComponent Object Reference"))
  ;[0.51 1 0.9801] Mouse Hover Functions
  (bind _asplayer_controller_bp (cast `/Game/Blueprints/Player/PlayerController_BP` (`GameplayStatics.GetPlayerController` 0)))
  (`/Game/Blueprints/Player/PlayerController_BP.UpdatePartHoveredOver` _asplayer_controller_bp self true))

(event `self.Part.OnEndCursorOver`
  (params (TouchedComponent :type "PrimitiveComponent Object Reference"))
  ;[0.51 1 0.9801] Mouse Hover Functions
  (bind _asplayer_controller_bp (cast `/Game/Blueprints/Player/PlayerController_BP` (`GameplayStatics.GetPlayerController` 0)))
  (`/Game/Blueprints/Player/PlayerController_BP.UpdatePartHoveredOver` _asplayer_controller_bp null false))

(event `AttachPart`
  ;[0.3742 0.724 0.353] Attach part
  (set `self.IsAttachedtoMouse` false)
  (set `self.CursorIsHovering` false))

(fn `UserConstructionScript`)