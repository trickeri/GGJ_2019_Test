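; Level transition trigger actor that fades out and loads another level when the player character overlaps it.
; On overlap, ChangeLevel flags the player as changing levels, plays a FadeOut level sequence at a configurable rate and binds an event to its finish.
; GetNextLevel switches on the LevelToLoad setting to open the matching map by name, covering the main menu and several gameplay and test levels.
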(event `self.ReceiveActorBeginOverlap`
  (params (OtherActor :type "Actor Object Reference"))
  ;[1 1 1] Level Change Overlap
  (if (== (`GameplayStatics.GetObjectClass` OtherActor) "/Game/Blueprints/Player/PlayerCharacter_BP.PlayerCharacter_BP_C")
    (bind _asplayer_character_bp (cast `/Game/Blueprints/Player/PlayerCharacter_BP` OtherActor))
    (`self.ChangeLevel` _asplayer_character_bp)))

(event `GetNextLevel`
  ;[1 1 1] Switch based on which level is set
  (switch `/Game/Blueprints/Environment/Enum_LevelChange` (`self.LevelToLoad`)
    (:`NewEnumerator0`
      (`GameplayStatics.OpenLevel` "MainMenu"))
    (:`NewEnumerator1`
      (`GameplayStatics.OpenLevel` "TheBasement"))
    (:`NewEnumerator2`
      (`GameplayStatics.OpenLevel` "TestLevel_1"))
    (:`NewEnumerator3`
      (`GameplayStatics.OpenLevel` "CombatLevel_1"))
    (:`NewEnumerator4`
      (`GameplayStatics.OpenLevel` "CombatLevel1"))))

(event `ChangeLevel`
  (params (PlayerCharacter :type "/Game/Blueprints/Player/PlayerCharacter_BP Object Reference"))
  ;[1 1 1] Level Change Overlap
  (set `GGJ_2019_TestCharacter.isChangingLevels` true PlayerCharacter)
  (bind (_outactor _returnvalue) (`LevelSequencePlayer.CreateLevelSequencePlayer` "/Game/Sequencer/FadeOut.FadeOut" (make `MovieSceneSequencePlaybackSettings` 0 (`self.FadeOutRate`))))
  (`MovieSceneSequencePlayer.Play` _returnvalue)
  (add `MovieSceneSequencePlayer.OnFinished` _returnvalue (`|CreateDelegate` :!event `GetNextLevel`)))

(fn `UserConstructionScript`)