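; Exploration-mode controller that, on BeginPlay, restores the player's saved location after combat and spawns enemies at ExplorationEnemySpawnPoint actors.
; Spawn points whose object names appear in the GameInstance's DefeatedEnemySpawns are marked killed.
; Killed points are skipped only when returning from a won fight, which also clears both combat flags; otherwise every point spawns.
; Only Melee Creep is handled, and each enemy stores its spawn point.
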(event `self.ReceiveBeginPlay`
  (bind _gameinstanceref (`self.GameInstanceRef`))
  (bind _gameinstanceref_2 (`self.GameInstanceRef`))
  ;[1 1 1] BeginPlay and Grab GameInstance Ref
  (bind _asgame_instance_bp (cast `/Game/Blueprints/General/GameInstance_BP` (`GameplayStatics.GetGameInstance`)))
  (set `self.GameInstanceRef` _asgame_instance_bp)
  (`|ExecutionSequence`
    (:`then_0`
      ;[1 1 1] Spawn player at a different location if they are exiting combat
      (if (`/Game/Blueprints/General/GameInstance_BP.PlayerIsReturningFromCombat` _gameinstanceref_2)
        (`self.K2_SetActorLocation` (`Controller.K2_GetPawn` (`GameplayStatics.GetPlayerController` 0)) (.location (`/Game/Blueprints/General/GameInstance_BP.PlayerExplorationLocation` _gameinstanceref_2)) false false)))
    (:`then_1`
      ;[1 1 1] Set the array of enemy spawn points
      (bind _outactors (`GameplayStatics.GetAllActorsOfClass` "/Game/Blueprints/Enemies/ExplorationModeSpawns/ExplorationEnemySpawnPoint.ExplorationEnemySpawnPoint_C"))
      (bind _output_get (set `self.EnemySpawnPoints` _outactors))
      (for _array_element _output_get
        (for _array_element_2 (`/Game/Blueprints/General/GameInstance_BP.DefeatedEnemySpawns` (`self.GameInstanceRef`))
          (if (`KismetStringLibrary.EqualEqual_StrStr` (`KismetSystemLibrary.GetObjectName` _array_element) _array_element_2)
            (set `/Game/Blueprints/Enemies/ExplorationModeSpawns/ExplorationEnemySpawnPoint.EnemyWasKilled` true _array_element)))))
    (:`then_2`
      ;[1 1 1] Spawn enemies accordingly
      (if (and (`/Game/Blueprints/General/GameInstance_BP.PlayerIsReturningFromCombat` _gameinstanceref) (`/Game/Blueprints/General/GameInstance_BP.PlayerDefeatedEnemies` _gameinstanceref))
        (set `/Game/Blueprints/General/GameInstance_BP.PlayerIsReturningFromCombat` false _gameinstanceref)
        (set `/Game/Blueprints/General/GameInstance_BP.PlayerDefeatedEnemies` false _gameinstanceref)
        (for _array_element_3 (`self.EnemySpawnPoints`)
          (if (not (`/Game/Blueprints/Enemies/ExplorationModeSpawns/ExplorationEnemySpawnPoint.EnemyWasKilled` _array_element_3))
            (switch `/Game/Blueprints/Enemies/ExplorationModeSpawns/EnemySpawnType` (`/Game/Blueprints/Enemies/ExplorationModeSpawns/ExplorationEnemySpawnPoint.EnemyTypeToSpawn` _array_element_3)
              (:`NewEnumerator0`
                (bind _returnvalue (`|SpawnActorFromClass` "/Game/Blueprints/Enemies/ExplorationModeSpawns/ExplorationModeEnemy_BP.ExplorationModeEnemy_BP_C" (`self.GetTransform` _array_element_3) "Undefined" "OverrideRootScale" null (struct) null))
                (set `/Game/Blueprints/Enemies/ExplorationModeSpawns/ExplorationModeEnemy_BP.AssignedSpawnPoint` _array_element_3 _returnvalue)))))
        (else
          (for _array_element_4 (`self.EnemySpawnPoints`)
            (switch `/Game/Blueprints/Enemies/ExplorationModeSpawns/EnemySpawnType` (`/Game/Blueprints/Enemies/ExplorationModeSpawns/ExplorationEnemySpawnPoint.EnemyTypeToSpawn` _array_element_4)
              (:`NewEnumerator0`
                (bind _returnvalue_2 (`|SpawnActorFromClass` "/Game/Blueprints/Enemies/ExplorationModeSpawns/ExplorationModeEnemy_BP.ExplorationModeEnemy_BP_C" (`self.GetTransform` _array_element_4) "Undefined" "OverrideRootScale" null (struct) null))
                (set `/Game/Blueprints/Enemies/ExplorationModeSpawns/ExplorationModeEnemy_BP.AssignedSpawnPoint` _array_element_4 _returnvalue_2)))))))))

(fn `UserConstructionScript`)