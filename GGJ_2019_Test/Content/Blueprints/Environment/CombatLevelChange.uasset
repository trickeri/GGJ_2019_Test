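; Environment Blueprint that moves the player from exploration into a combat level, with ChangeLevel as its entry point.
; ChangeLevel flags the player as changing levels, stores their transform in the game instance, and plays a fade-out Level Sequence with a completion callback.
; GetNextLevel opens CombatLevel_1 by a hardcoded name, with no branching on level choice yet.
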(event `self.ReceiveBeginPlay`
  ;[1 1 1] BeginPlay
  (bind _asgame_instance_bp (cast `/Game/Blueprints/General/GameInstance_BP` (`GameplayStatics.GetGameInstance`)))
  (set `self.GameInstanceRef` _asgame_instance_bp))

(event `ChangeLevel`
  (params (PlayerCharacter :type "/Game/Blueprints/Player/PlayerCharacter_BP Object Reference"))
  ;[1 1 1] Level Change Overlap
  (set `GGJ_2019_TestCharacter.isChangingLevels` true PlayerCharacter)
  (set `/Game/Blueprints/General/GameInstance_BP.PlayerExplorationLocation` (`self.GetTransform` PlayerCharacter) (`self.GameInstanceRef`))
  (bind (_outactor _returnvalue) (`LevelSequencePlayer.CreateLevelSequencePlayer` "/Game/Sequencer/FadeOut.FadeOut" (make `MovieSceneSequencePlaybackSettings` 0 (`self.FadeOutRate`))))
  (`MovieSceneSequencePlayer.Play` _returnvalue)
  (add `MovieSceneSequencePlayer.OnFinished` _returnvalue (`|CreateDelegate` :!event `GetNextLevel`)))

(event `GetNextLevel`
  ;[1 1 1] Switch based on which level is set
  (`GameplayStatics.OpenLevel` "CombatLevel_1"))

(fn `UserConstructionScript`)